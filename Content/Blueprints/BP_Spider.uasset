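; Spider actor that wanders over surrounding geometry, alternating random idle waits with short walks, until damage kills it.
; A Tick-driven state machine runs Idle, Walking and Dying.
; TracePath fans line traces from an elevated, ceiling-clamped probe along a random horizontal direction, storing hit points and normals that Walking interpolates to move and align the spider to surfaces.
; Dying ramps a dissolve parameter on a dynamic material, then destroys the actor.
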(event `self.ReceiveTick`
  (params (DeltaSeconds :type "Float (single-precision)"))
  (switch `/Game/Blueprints/Enums/E_EnemyState` (`self.CurrentState`)
    (:`NewEnumerator0`
      (`self.OnIdle` DeltaSeconds))
    (:`NewEnumerator1`
      (`self.OnWalking` DeltaSeconds))
    (:`NewEnumerator2`
      (`self.OnDying` DeltaSeconds))))

(event `self.ReceiveBeginPlay`
  (bind _mesh (`self.Mesh`))
  (bind _returnvalue (`PrimitiveComponent.CreateDynamicMaterialInstance` _mesh 0 (`PrimitiveComponent.GetMaterial` _mesh 0) "None"))
  (set `self.MaterialInstance` _returnvalue)
  (set `self.IdleWaitTimer` (`KismetMathLibrary.RandomFloatInRange` 0.0 (`self.MaximumIdleWait`))))

(event `self.ReceiveAnyDamage`
  (params (Damage :type "Float (single-precision)") (DamageType :type "DamageType Object Reference") (InstigatedBy :type "Controller Object Reference") (DamageCauser :type "Actor Object Reference"))
  (if (> (`self.Health`) 0.0)
    (bind _output_get (set `self.Health` (- (`self.Health`) Damage)))
    (if (<= _output_get 0.0)
      (set `self.CurrentState` "NewEnumerator2"))))

(fn `OnDying`
  (params (DeltaSeconds :type "Float (double-precision)"))
  (bind _output_get (set `self.DissolveAmount` (+ DeltaSeconds (`self.DissolveAmount`))))
  (`MaterialInstanceDynamic.SetScalarParameterValue` (`self.MaterialInstance`) "DissolveAmount" (`KismetMathLibrary.FMin` _output_get 1.0))
  (if (>= (`self.DissolveAmount`) 1.0)
    (`self.K2_DestroyActor`)))

(fn `OnIdle`
  (params (DeltaSeconds :type "Float (double-precision)"))
  (bind _output_get (set `self.IdleWaitTimer` (- (`self.IdleWaitTimer`) DeltaSeconds)))
  (if (<= _output_get 0.0)
    (`self.TracePath`)
    (set `self.CurrentState` "NewEnumerator1")
    (return)
    (else
      (return))))

(fn `OnWalking`
  (params (DeltaSeconds :type "Float (double-precision)"))
  (bind _walktargets (`self.WalkTargets`))
  (bind _walktargetnormals (`self.WalkTargetNormals`))
  (bind _output_get (set `self.WalkTargetIndex` (+ (`self.WalkTargetIndex`) (* DeltaSeconds (`self.WalkSpeed`)))))
  (if (>= (`KismetMathLibrary.FFloor` _output_get) (- (`KismetArrayLibrary.Array_Length` (`self.WalkTargets`)) 1))
    (set `self.CurrentState` "NewEnumerator0")
    (set `self.IdleWaitTimer` (`KismetMathLibrary.RandomFloatInRange` 0.0 (`self.MaximumIdleWait`)))
    (else
      (bind _returnvalue (`KismetMathLibrary.FFloor` _output_get))
      (bind _output (`|GetArrayItem` _walktargets _returnvalue))
      (bind _returnvalue_2 (`KismetMathLibrary.FCeil` _output_get))
      (bind _output_2 (`|GetArrayItem` _walktargets _returnvalue_2))
      (bind _returnvalue_3 (`KismetMathLibrary.Fraction` _output_get))
      (`self.K2_SetActorLocation` (`KismetMathLibrary.VLerp` _output _output_2 _returnvalue_3))
      (bind _returnvalue_4 (`KismetMathLibrary.Normal` (- _output_2 _output)))
      (`self.K2_SetActorRotation` (`KismetMathLibrary.RLerp` (`KismetMathLibrary.MakeRotFromZX` (`|GetArrayItem` _walktargetnormals _returnvalue) _returnvalue_4) (`KismetMathLibrary.MakeRotFromZX` (`|GetArrayItem` _walktargetnormals _returnvalue_2) _returnvalue_4) _returnvalue_3)))))

(fn `TracePath`
  (locals (WalkDirection :type "Vector Structure") (ProbeLocation :type "Vector Structure") (ProbeTarget :type "Vector Structure") (ProbeSteps :type Integer))
  (bind (_returnvalue_x _returnvalue_y) (`KismetMathLibrary.BreakVector` (`KismetMathLibrary.RandomUnitVector`)))
  (bind _returnvalue (`SceneComponent.K2_GetComponentLocation` (`self.PathTraceProbe`)))
  (`KismetArrayLibrary.Array_Clear` (`self.WalkTargets`))
  (`KismetArrayLibrary.Array_Clear` (`self.WalkTargetNormals`))
  (set `local.WalkDirection` (`KismetMathLibrary.Normal` (`KismetMathLibrary.MakeVector` _returnvalue_x _returnvalue_y)))
  (bind _output_get (set `local.ProbeLocation` (+ _returnvalue (0.0 0.0 1000.0))))
  ;[1 1 1] Keeps the probe under ceilings...
  (bind (_outhit _returnvalue_2) (`KismetSystemLibrary.LineTraceSingleForObjects` _output_get _returnvalue (`self.ObjectTypesToTrace`) true))
  (if _returnvalue_2
    (set `local.ProbeLocation` (- (`.Location` (`GameplayStatics.BreakHitResult` _outhit)) (0.0 0.0 10.0))))
  (for _index (range (+ (`KismetMathLibrary.FCeil` (/ (`KismetMathLibrary.RandomFloatInRange` (`self.WalkStepResolution`) (`self.MaxWalkDistance`)) (`self.WalkStepResolution`))) 1))
    (bind (_outhit_2 _returnvalue_3) (`KismetSystemLibrary.LineTraceSingleForObjects` (`local.ProbeLocation`) (+ (* (* (`local.WalkDirection`) (`KismetMathLibrary.Conv_IntToDouble` _index)) (`self.WalkStepResolution`)) (`self.K2_GetActorLocation`) (0.0 0.0 -200.0)) (`self.ObjectTypesToTrace`) true))
    (if _returnvalue_3
      (`KismetArrayLibrary.Array_Add` (`self.WalkTargets`) (`.Location` (`GameplayStatics.BreakHitResult` _outhit_2)))
      (`KismetArrayLibrary.Array_Add` (`self.WalkTargetNormals`) (`.Normal` (`GameplayStatics.BreakHitResult` _outhit_2)))))
  (set `self.WalkTargetIndex` 0.0))

(fn `UserConstructionScript`)