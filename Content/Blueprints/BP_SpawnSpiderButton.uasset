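; BP_SpawnSpiderButton is a button actor that spawns an actor, a spider going by the asset name, when pressed.
; On the button component's press event, it traces straight down on the Visibility channel from a point behind the button.
; If the trace hits, it spawns at the hit location, upright and aligned to the button's forward vector, with the player pawn as instigator.
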(event `self.ButtonComponent.OnButtonPressed`
  (params (Button :type "UxtPressableButtonComponent Object Reference") (Pointer :type "UxtPointerComponent Object Reference"))
  (bind _returnvalue (`self.GetActorForwardVector`))
  (bind _returnvalue_2 (+ (`self.K2_GetActorLocation`) (* (`KismetMathLibrary.NegateVector` _returnvalue) 200.0)))
  (bind (_outhit _returnvalue_3) (`KismetSystemLibrary.LineTraceSingle` _returnvalue_2 (- _returnvalue_2 (0.0 0.0 2000.0)) "TraceTypeQuery1"))
  (if _returnvalue_3
    (`|SpawnActorFromClass` "/Game/Blueprints/BP_Spider.BP_Spider_C" (`KismetMathLibrary.MakeTransform` (`.Location` (`GameplayStatics.BreakHitResult` _outhit)) (`KismetMathLibrary.MakeRotFromZX` (`KismetMathLibrary.Vector_Up`) _returnvalue)) "Undefined" "OverrideRootScale" null (`GameplayStatics.GetPlayerPawn` 0))))

(fn `UserConstructionScript`)