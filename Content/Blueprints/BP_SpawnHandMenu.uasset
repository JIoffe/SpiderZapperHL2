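; BP_SpawnHandMenu is a mixed reality hand menu that appears and hides with a UX Tools palm-up constraint.
; Activation shows the UI element, notifies MRPawn and spawns a right-hand UxtHandInteractionActor owned by the player pawn.
; Deactivation hides the UI, notifies the pawn and destroys that actor, so this right-hand interaction actor exists only while the menu is up.
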(event `self.UxtPalmUpConstraint.OnConstraintActivated`
  (bind _returnvalue (`GameplayStatics.GetPlayerPawn` 0))
  (`UxtUIElementComponent.SetUIVisibility` (`self.UxtUIElement`) "Show")
  (bind _asmrpawn (cast `/Game/MRPawn` _returnvalue))
  (`/Game/MRPawn.OnMenuShow` _asmrpawn)
  (bind _returnvalue_2 (`|SpawnActorFromClass` "/Script/UXTools.UxtHandInteractionActor" (`KismetMathLibrary.MakeTransform` (0.0 0.0 0.0)) "Undefined" "OverrideRootScale" _returnvalue false "Right" null))
  (set `self.RightHandInteraction` _returnvalue_2))

(event `self.UxtPalmUpConstraint.OnConstraintDeactivated`
  (bind _righthandinteraction (`self.RightHandInteraction`))
  (`UxtUIElementComponent.SetUIVisibility` (`self.UxtUIElement`) "Hide")
  (bind _asmrpawn (cast `/Game/MRPawn` (`GameplayStatics.GetPlayerPawn` 0)))
  (`/Game/MRPawn.OnMenuHide` _asmrpawn)
  (`/Engine/EditorBlueprintResources/StandardMacros.IsValid` _righthandinteraction
    (:`Is Valid`
      (`self.K2_DestroyActor` _righthandinteraction)
      (set `self.RightHandInteraction` null))))

(fn `UserConstructionScript`)