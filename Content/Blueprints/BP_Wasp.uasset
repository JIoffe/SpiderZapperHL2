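; BP_Wasp is a damageable wasp actor that hovers around its spawn point until killed, then falls and dissolves away.
; While Idle or Walking, Tick offsets it from its initial location with sine waves along the up and right axes.
; Lethal damage enables mesh physics and switches to Dying, where the actor follows the mesh and raises DissolveAmount on dynamic materials created at BeginPlay before destroying itself.
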(event `self.ReceiveBeginPlay`
  (bind _mesh (`self.Mesh`))
  (set `self.InitialPosition` (`self.K2_GetActorLocation`))
  (for _index (range 3)
    (bind _returnvalue (`PrimitiveComponent.CreateDynamicMaterialInstance` _mesh _index (`PrimitiveComponent.GetMaterial` _mesh _index) "None"))
    (`KismetArrayLibrary.Array_Add` (`self.MaterialInstances`) _returnvalue)))

(event `self.ReceiveTick`
  (params (DeltaSeconds :type "Float (single-precision)"))
  (switch `/Game/Blueprints/Enums/E_EnemyState` (`self.CurrentState`)
    (:`NewEnumerator0`
      (`self.DoHover` :!label _label))
    (:`NewEnumerator1`
      (goto _label))
    (:`NewEnumerator2`
      (`self.OnDying` DeltaSeconds))))

(event `self.ReceiveAnyDamage`
  (params (Damage :type "Float (single-precision)") (DamageType :type "DamageType Object Reference") (InstigatedBy :type "Controller Object Reference") (DamageCauser :type "Actor Object Reference"))
  (if (> (`self.Health`) 0.0)
    (bind _output_get (set `self.Health` (- (`self.Health`) Damage)))
    (if (<= _output_get 0.0)
      (set `self.CurrentState` "NewEnumerator2")
      (`PrimitiveComponent.SetSimulatePhysics` (`self.Mesh`) true))))

(fn `DoHover`
  (bind _returnvalue (`self.GetGameTimeSinceCreation`))
  (bind (_hoverspeed_x _hoverspeed_y) (`KismetMathLibrary.BreakVector2D` (`self.HoverSpeed`)))
  (bind (_hoveroffset_x _hoveroffset_y) (`KismetMathLibrary.BreakVector2D` (`self.HoverOffset`)))
  (`self.K2_SetActorLocation` (+ (`self.InitialPosition`) (* (`KismetMathLibrary.Vector_Up`) (* (`KismetMathLibrary.Sin` (* _returnvalue _hoverspeed_y)) _hoveroffset_y)) (* (`self.GetActorRightVector`) (* (`KismetMathLibrary.Sin` (* _returnvalue _hoverspeed_x)) _hoveroffset_x)))))

(fn `OnDying`
  (params (DeltaSeconds :type "Float (double-precision)"))
  (bind _output_get (set `self.DissolveAmount` (+ (* DeltaSeconds 0.5) (`self.DissolveAmount`))))
  (`self.K2_SetActorLocation` (`SceneComponent.K2_GetComponentLocation` (`self.Mesh`)))
  (for _array_element (`self.MaterialInstances`)
    (`MaterialInstanceDynamic.SetScalarParameterValue` _array_element "DissolveAmount" (`KismetMathLibrary.FMin` _output_get 1.0)))
  (if (>= (`self.DissolveAmount`) 1.0)
    (`self.K2_DestroyActor`)))

(fn `UserConstructionScript`)